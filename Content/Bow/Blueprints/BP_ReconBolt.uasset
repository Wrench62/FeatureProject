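; Recon bolt projectile for the bow that bounces up to a set limit, sticks, then scans for targets in pulses.
; Charge strength sets launch speed and gravity scale.
; After a windup, a looping timer grows a sphere trace, line-traces each hit for cover and notifies visible BPI_Scannable actors.
; Scans repeat before the bolt destroys itself, but progress stalls when every detected target is blocked (noted bug).
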(event `StartMove`
  (params (Strength :type "Float (double-precision)") (Bounce :type Integer) (Direction :type "Vector Structure"))
  ; Sets Velocity and Gravity based on Strength Alpha charge value
  (set `MovementComponent.Velocity` (* Direction (`KismetMathLibrary.Lerp` (`self.MinSpeed`) (`self.MaxSpeed`) Strength)) (`self.ProjectileMovement`))
  (set `ProjectileMovementComponent.ProjectileGravityScale` (`KismetMathLibrary.Lerp` (`self.MaxGravity`) (`self.MinGravity`) Strength) (`self.ProjectileMovement`))
  (set `self.Bounce` Bounce)
  ; Checks if bounce is set to 0, if so, disables bounce
  (if (== (`self.Bounce`) 0)
    (set `ProjectileMovementComponent.bShouldBounce` false (`self.ProjectileMovement`))))

(event `self.ProjectileMovement.OnProjectileBounce`
  (params (ImpactResult :type "HitResult Structure (by ref)") (ImpactVelocity :type "Vector Structure (by ref)"))
  ; After every bounce, checks if bounce limit has been hit, if so, stop bouncing and stick
  (bind _result (`/Engine/EditorBlueprintResources/StandardMacros.IncrementInt` (`self.BounceCount`))
    (:`  `
      (if (>= _result (`self.Bounce`))
        (set `ProjectileMovementComponent.bShouldBounce` false (`self.ProjectileMovement`))))))

(event `self.ProjectileMovement.OnProjectileStop`
  (params (ImpactResult :type "HitResult Structure (by ref)"))
  (`KismetSystemLibrary.Delay` 0.667) ; Windup Delay
  (bind _returnvalue (`KismetSystemLibrary.K2_SetTimerDelegate` (delegate `Initial Sphere Scan`) (`self.TimeIncrement`) true :!label _label))
  (set `self.TimerRef` _returnvalue))

(event `Initial Sphere Scan`
  (bind _returnvalue (`self.K2_GetActorLocation`))
  (bind (_outhits _returnvalue_2) (`KismetSystemLibrary.SphereTraceMultiForObjects` :`Start` _returnvalue :`End` _returnvalue :`Radius` (`self.Radius`) :`ObjectTypes` (`self.ObjectTypes1`) :`DrawDebugType` "ForDuration" :`TraceColor` (struct :`R` 0.3564 :`G` 0.887923 :`B` 0.930111 :`A` 1.0) :`TraceHitColor` (struct :`G` 0.856813 :`B` 1.0 :`A` 1.0) :`DrawTime` 0.3))
  (if _returnvalue_2
    ; For each enemy scanned, check if there's anything between the recon bolt and the enemy
    (for _array_element _outhits
      (bind _outhit (`KismetSystemLibrary.LineTraceSingleForObjects` :`Start` (`self.K2_GetActorLocation`) :`End` (`self.K2_GetActorLocation` (`.HitActor` (`GameplayStatics.BreakHitResult` _array_element))) :`ObjectTypes` (`self.ObjectTypes2`) :`bTraceComplex` true :`DrawDebugType` "ForDuration" :`DrawTime` 2.0))
      (bind (_bblockinghit _binitialoverlap _time _distance _location _impactpoint _normal _impactnormal _physmat _hitactor) (`GameplayStatics.BreakHitResult` _outhit))
      ; If not, the target is scanned
      (if (`KismetSystemLibrary.DoesImplementInterface` _hitactor "/Game/Enemy/Blueprints/BPI_Scannable.BPI_Scannable_C")
        (message `/Game/Enemy/Blueprints/BPI_Scannable.OnScanned` _hitactor self)
        (bind _output_get (set `self.Time` (+ (`self.Time`) (`self.TimeIncrement`)) :!label _label_2))
        (set `self.Radius` (`KismetMathLibrary.Lerp` (`self.MinRadius`) (`self.MaxRadius`) (`KismetMathLibrary.FClamp` (`KismetMathLibrary.NormalizeToRange` _output_get 0.0 (`self.MaxTime`)))))
        (if (>= (`self.Time`) (`self.MaxTime`))
          (`KismetSystemLibrary.K2_ClearAndInvalidateTimerHandle` (`self.TimerRef`))
          (set `self.Time` 0.0)
          (set `self.Radius` (`self.MinRadius`))
          (if (>= (`self.ScanCounter`) 2)
            (`KismetSystemLibrary.PrintString` "Scan 2 Complete!")
            (`self.OnFinishedScanning`)
            (`KismetSystemLibrary.Delay` 0.2)
            (`self.K2_DestroyActor`)
            (else
              (`/Engine/EditorBlueprintResources/StandardMacros.IncrementInt` (`self.ScanCounter`)
                (:`  `
                  (`KismetSystemLibrary.PrintString` "Scan 1 Complete")
                  (`self.OnFinishedScanning`)
                  (goto _label))))))
        (else
          ; BUG: If no target can be scanned (is behind wall). code gets stuck here.
          (`KismetSystemLibrary.PrintString` "no enemies scanned!"))))
    (else
      (goto _label_2))))

(fn `UserConstructionScript`)